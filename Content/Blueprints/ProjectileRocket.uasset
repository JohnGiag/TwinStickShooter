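; Rocket projectile actor that explodes on overlap, damaging non-friendly targets.
; Damageable actors without the Friendly tag receive an IDamageable health message, then the rocket applies full-strength radial damage with a negative base value.
; Non-damageable overlaps skip straight to the explosion sound, particle effect and self-destruction.
; Friendly damageable actors are ignored, leaving the rocket intact.
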(event `self.ReceiveTick`
  (params (DeltaSeconds :type "Float (single-precision)")))

(event `self.ReceiveBeginPlay`)

(event `self.ReceiveActorBeginOverlap`
  (params (OtherActor :type "Actor Object Reference"))
  (bind (_returnvalue_location _returnvalue_rotation) (`KismetMathLibrary.BreakTransform` (`self.GetTransform`)))
  (if (`KismetSystemLibrary.DoesImplementInterface` OtherActor "/Game/Blueprints/iDamageable.iDamageable_C")
    (if (not (`self.ActorHasTag` OtherActor "Friendly"))
      (message `/Game/Blueprints/iDamageable.AffectHealth` OtherActor (`self.Damage`))
      (`GameplayStatics.ApplyRadialDamage` :`BaseDamage` -150.0 :`Origin` (`SceneComponent.K2_GetComponentLocation` (`self.Rocket Collision`)) :`DamageRadius` 1000.0 :`bDoFullDamage` true :`DamagePreventionChannel` "ECC_Vehicle")
      (`GameplayStatics.PlaySoundAttached` "/Game/Meshes/Rocket/Explosion_sound.Explosion_sound" (`self.Rocket Collision`) :!label _label)
      (`GameplayStatics.SpawnEmitterAtLocation` "/Game/StarterContent/Particles/P_Explosion.P_Explosion" _returnvalue_location _returnvalue_rotation)
      (`self.K2_DestroyActor`))
    (else
      (goto _label))))

(fn `UserConstructionScript`)