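; Turret spawn manager that respawns an EnemyTurretGun at one of five random points when none exist in the level.
; Each Tick searches all actors for that class, and an empty result starts a 15-second Delay.
; A random integer switch then spawns the turret at the world transform of one of five scene components, with the default branch covering the fifth.
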(event `self.ReceiveActorBeginOverlap`
  (params (OtherActor :type "Actor Object Reference")))

(event `self.ReceiveTick`
  (params (DeltaSeconds :type "Float (single-precision)"))
  (bind _outactors (`GameplayStatics.GetAllActorsOfClass` "/Game/Blueprints/EnemyTurretGun.EnemyTurretGun_C"))
  (if (== (`KismetArrayLibrary.Array_Length` _outactors) 0)
    (`KismetSystemLibrary.Delay` 15.0)
    (switch `int` (`KismetMathLibrary.RandomIntegerInRange` 0 4)
      (:`Default`
        (`|SpawnActorFromClass` "/Game/Blueprints/EnemyTurretGun.EnemyTurretGun_C" (`SceneComponent.K2_GetComponentToWorld` (`self.SceneComp4`))))
      (:`0`
        (`|SpawnActorFromClass` "/Game/Blueprints/EnemyTurretGun.EnemyTurretGun_C" (`SceneComponent.K2_GetComponentToWorld` (`self.SceneComp`))))
      (:`1`
        (`|SpawnActorFromClass` "/Game/Blueprints/EnemyTurretGun.EnemyTurretGun_C" (`SceneComponent.K2_GetComponentToWorld` (`self.SceneComp1`))))
      (:`2`
        (`|SpawnActorFromClass` "/Game/Blueprints/EnemyTurretGun.EnemyTurretGun_C" (`SceneComponent.K2_GetComponentToWorld` (`self.SceneComp2`))))
      (:`3`
        (`|SpawnActorFromClass` "/Game/Blueprints/EnemyTurretGun.EnemyTurretGun_C" (`SceneComponent.K2_GetComponentToWorld` (`self.SceneComp3`)))))))

(fn `UserConstructionScript`)