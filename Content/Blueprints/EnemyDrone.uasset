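; EnemyDrone is a twin-stick shooter enemy that fires at the player when in range and awards score on death.
; Each Tick compares player distance to AttackRange, with a Delay throttling projectile spawns from two gun sockets on the drone.
; AffectHealth applies health deltas; at zero or below it drops WorldStatic and Pawn collision, increments TwinStickMode score, detaches its controller, then spawns an explosion and destroys itself.
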(event `self.ReceiveBeginPlay`)

(event `self.ReceiveActorBeginOverlap`
  (params (OtherActor :type "Actor Object Reference")))

(event `self.ReceiveTick`
  (params (DeltaSeconds :type "Float (single-precision)"))
  (`self.UpdateRange`)
  (`self.Fire`))

(event `UpdateRange`
  ;[1 1 1] Update Range
  (if (< (`self.GetDistanceTo` self (`GameplayStatics.GetPlayerCharacter` 0)) (`self.AttackRange`))
    (set `self.Enemy In Range ?` true)
    (else
      (set `self.Enemy In Range ?` false))))

(event `/Game/Blueprints/iDamageable.AffectHealth`
  (params (Delta :type "Float (single-precision)"))
  (bind _capsulecomponent (`self.CapsuleComponent`))
  ;[1 1 1] Handle Death
  (bind _output_get (set `self.Health` (+ Delta (`self.Health`))))
  (if (<= _output_get 0.0)
    (set `self.Is Dead` true)
    (else
      (set `self.Is Dead` false)))
  (if (`self.Is Dead`)
    (`PrimitiveComponent.SetCollisionResponseToChannel` _capsulecomponent "ECC_WorldStatic" "ECR_Ignore")
    (`PrimitiveComponent.SetCollisionResponseToChannel` _capsulecomponent "ECC_Pawn" "ECR_Ignore")
    (bind _astwin_stick_mode (cast `/Game/Blueprints/TwinStickMode` (`GameplayStatics.GetGameMode`)))
    (`/Game/Blueprints/TwinStickMode.Increment Score` _astwin_stick_mode (`self.Score`))
    (`self.DetachFromControllerPendingDestroy`)
    (`KismetSystemLibrary.Delay` 0.2)
    (`|SpawnActorFromClass` "/Game/Blueprints/Explosion.Explosion_C" (`self.GetTransform`))
    (`self.K2_DestroyActor`)))

(event `Fire`
  (bind _drone (`self.Drone`))
  ;[1 1 1] Fire
  (if (`self.Enemy In Range ?`)
    (`KismetSystemLibrary.Delay` (`self.FireInterval`))
    (`|SpawnActorFromClass` "/Game/Blueprints/EnemyDroneProjectile.EnemyDroneProjectile_C" (`SceneComponent.GetSocketTransform` _drone "g1" "RTS_World"))
    (`|SpawnActorFromClass` "/Game/Blueprints/EnemyDroneProjectile.EnemyDroneProjectile_C" (`SceneComponent.GetSocketTransform` _drone "g2" "RTS_World"))))

(fn `UserConstructionScript`)