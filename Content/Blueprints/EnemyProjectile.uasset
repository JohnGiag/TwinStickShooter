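; EnemyProjectile is an enemy laser projectile that damages friendly targets on overlap.
; Damageable actors tagged Friendly receive its Damage through the IDamageable AffectHealth message, followed by an attached hit sound, a spark emitter and self-destruction.
; Actors without the interface trigger the same impact and destruction without damage, while damageable actors lacking the tag are ignored.
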(event `self.ReceiveBeginPlay`)

(event `self.ReceiveActorBeginOverlap`
  (params (OtherActor :type "Actor Object Reference"))
  (bind (_returnvalue_location _returnvalue_rotation) (`KismetMathLibrary.BreakTransform` (`self.GetTransform`)))
  (if (`KismetSystemLibrary.DoesImplementInterface` OtherActor "/Game/Blueprints/iDamageable.iDamageable_C")
    (if (`self.ActorHasTag` OtherActor "Friendly")
      (message `/Game/Blueprints/iDamageable.AffectHealth` OtherActor (`self.Damage`))
      (`GameplayStatics.PlaySoundAttached` "/Game/Audio/LaserHit.LaserHit" (`self.Projectile Collision`) :!label _label)
      (`GameplayStatics.SpawnEmitterAtLocation` "/Game/StarterContent/Particles/EnemyLaserSparks.EnemyLaserSparks" _returnvalue_location _returnvalue_rotation)
      (`self.K2_DestroyActor`))
    (else
      (goto _label))))

(event `self.ReceiveTick`
  (params (DeltaSeconds :type "Float (single-precision)")))

(fn `UserConstructionScript`)