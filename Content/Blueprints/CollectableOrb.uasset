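; CollectableOrb is a pickup that homes in on the player and expires after 15 seconds if uncollected.
; Each tick it eases toward the player pawn with an unswept VInterpTo.
; On overlap with an actor tagged Friendly, it calls OrbCount on the player HeroCharacter's Weapon and destroys itself.
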(event `self.ReceiveBeginPlay`
  (`self.SetLifeSpan` 15.0))

(event `self.ReceiveActorBeginOverlap`
  (params (OtherActor :type "Actor Object Reference"))
  (if (`self.ActorHasTag` OtherActor "Friendly")
    (bind _ashero_character (cast `/Game/Blueprints/HeroCharacter` (`GameplayStatics.GetPlayerCharacter` 0)))
    (`/Game/Blueprints/Weapon.OrbCount` (`/Game/Blueprints/HeroCharacter.Weapon` _ashero_character))
    (`self.K2_DestroyActor`)))

(event `self.ReceiveTick`
  (params (DeltaSeconds :type "Float (single-precision)"))
  (bind _returnvalue (`GameplayStatics.GetPlayerPawn` 0))
  ;[1 1 1] Orb moving towards the player
  (set `self.DeltaTime` DeltaSeconds)
  (`/Engine/EditorBlueprintResources/StandardMacros.IsValid` _returnvalue
    (:`Is Valid`
      (`self.K2_SetActorLocation` (`KismetMathLibrary.VInterpTo` (`self.K2_GetActorLocation`) (`self.K2_GetActorLocation` _returnvalue) (`self.DeltaTime`) 1.0)))))

(fn `UserConstructionScript`)