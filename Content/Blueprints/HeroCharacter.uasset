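; Player character for a twin-stick shooter, handling movement, aiming, shooting, rocket attack, pause menu and timed speed pickup.
; BeginPlay attaches a weapon, adds the HUD and gives TwinStickMode the spawn transform; death ends the game after a delay.
; Right-stick input rotates and fires, while Tick switches to cursor aiming on mouse movement and runs gated, delay-throttled mouse fire.
; A debug key builds a key-rebinding menu from Victory plugin bindings.
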(event `self.ReceiveBeginPlay`
  (bind _mesh (`self.Mesh`))
  (`|ExecutionSequence`
    (:`then_0`
      (bind _returnvalue (`|SpawnActorFromClass` "/Game/Blueprints/Weapon.Weapon_C" (`SceneComponent.K2_GetComponentToWorld` _mesh)))
      (bind _output_get (set `self.Weapon` _returnvalue))
      (`self.K2_AttachRootComponentTo` _output_get _mesh "GunSocket" "SnapToTarget" true))
    (:`then_1`
      (bind _astwin_stick_mode (cast `/Game/Blueprints/TwinStickMode` (`GameplayStatics.GetGameMode`)))
      (bind _output_get_2 (set `self.GameMode` _astwin_stick_mode))
      (set `/Game/Blueprints/TwinStickMode.PlayerSpawnTransform` (`self.GetTransform`) _output_get_2))
    (:`then_2`
      (set `self.MaxHealth` (`self.Health`))
      (bind _returnvalue_2 (`|CreateWidget` "/Game/UMG/HUD/TwinStickHUD.TwinStickHUD_C" (`GameplayStatics.GetPlayerController` 0)))
      (`UserWidget.AddToViewport` _returnvalue_2 0)
      (set `self.IsLoading?` false))))

(event `self.ReceiveActorBeginOverlap`
  (params (OtherActor :type "Actor Object Reference")))

(event `InputAxis|MoveUp`
  (params (AxisValue :type "Float (single-precision)"))
  ;[1 1 1] Movement
  (`self.AddMovementInput` (1.0 0.0 0.0) AxisValue))

(event `InputAxis|MoveRight`
  (params (AxisValue :type "Float (single-precision)"))
  ;[1 1 1] Movement
  (`self.AddMovementInput` (0.0 1.0 0.0) AxisValue))

(event `InputAxis|LookUp`
  (params (AxisValue :type "Float (single-precision)"))
  (bind _weapon (`self.Weapon`))
  ;[1 1 1] Rotation/shooting with keyboard/controler
  (bind _returnvalue (`KismetMathLibrary.MakeVector` AxisValue (stale `InputAxis|LookRight` AxisValue)))
  (bind _returnvalue_2 (`KismetMathLibrary.VSize` _returnvalue))
  (set `self.NewVar` _returnvalue_2 :!label _label)
  (if (> _returnvalue_2 0.25)
    (`Controller.SetControlRotation` (`self.GetController`) (`KismetMathLibrary.Conv_VectorToRotator` _returnvalue))
    (`/Game/Blueprints/Weapon.Pull Trigger` _weapon)
    (else
      (`/Game/Blueprints/Weapon.Release Trigger` _weapon))))

(event `InputAxis|LookRight`
  (params (AxisValue :type "Float (single-precision)"))
  ;[1 1 1] Rotation/shooting with keyboard/controler
  (goto _label))

(event `/Game/Blueprints/iDamageable.AffectHealth`
  (params (Delta :type "Float (single-precision)"))
  ;[1 1 1] Handle Death
  (`self.CalculateHealth` Delta)
  (if (`self.isDead`)
    (`self.K2_DestroyActor` (`self.Weapon`))
    (`self.DisableInput` null)
    (`KismetSystemLibrary.Delay` 3.0)
    (`/Game/Blueprints/TwinStickMode.EndGame` (`self.GameMode`))
    (`self.K2_DestroyActor` self)))

(event `InputAction|Pause Game`
  (bind _returnvalue (`GameplayStatics.GetPlayerController` 0))
  ;[1 1 1] Pause Game
  (:`Pressed`
    (`GameplayStatics.SetGamePaused` true)
    (`self.DisableInput` _returnvalue null)
    (set `PlayerController.bShowMouseCursor` true _returnvalue)
    (`WidgetBlueprintLibrary.SetInputMode_UIOnlyEx` _returnvalue)
    (bind _returnvalue_2 (`|CreateWidget` "/Game/UMG/Menus/InGameMenu.InGameMenu_C"))
    (`UserWidget.AddToViewport` _returnvalue_2 0)
    (`Widget.SetKeyboardFocus` (`/Game/UMG/Menus/InGameMenu.B_resume` _returnvalue_2))))

(event `SpeedPickUp`
  (bind _charactermovement (`Character.CharacterMovement` (`GameplayStatics.GetPlayerCharacter` 0)))
  ;[1 1 1] Speed Pick Up
  (if (== (`CharacterMovementComponent.MaxWalkSpeed` _charactermovement) 600.0)
    (set `CharacterMovementComponent.MaxWalkSpeed` 1500.0 _charactermovement))
  (`KismetSystemLibrary.RetriggerableDelay` 4.0)
  (set `CharacterMovementComponent.MaxWalkSpeed` 600.0 _charactermovement))

(event `Key|K`
  ;[1 1 1] Rebind debug
  (:`Pressed`
    (`self.Open Rebind Menu`)
    (for _array_element (`VictoryBPFunctionLibrary.VictoryGetAllActionKeyBindings`)
      (`self.AddKeyBindToUMG` _array_element))))

(event `InputAction|TestInput`
  ;[1 1 1] Test input for debug
  (:`Pressed`
    (`KismetSystemLibrary.PrintString` "This Is A Test")))

(event `InputAction|Aim`
  (bind _returnvalue (`GameplayStatics.GetPlayerController` 0))
  ;[1 1 1] Toggle Aim
  (:`Pressed`
    (if (`self.Is Aiming?`)
      (set `self.Is Aiming?` false)
      (set `PlayerController.bShowMouseCursor` false _returnvalue)
      (else
        (set `self.Is Aiming?` true)
        (set `PlayerController.bShowMouseCursor` true _returnvalue)))))

(event `self.ReceiveTick`
  (params (DeltaSeconds :type "Float (single-precision)"))
  (bind _returnvalue (`GameplayStatics.GetPlayerController` 0))
  (bind _weapon (`self.Weapon`))
  (bind (_deltax _deltay) (`PlayerController.GetInputMouseDelta` _returnvalue))
  (if (> (`self.NewVar`) 0.25)
    (set `self.Is Aiming?` false)
    ;[1 1 1] Set Rotation While aiming
    (set `PlayerController.bShowMouseCursor` false _returnvalue)
    (elif (or (> _deltax 0.0) (> _deltay 0.0))
      (set `self.Is Aiming?` true)
      (set `PlayerController.bShowMouseCursor` true _returnvalue)))
  (`|ExecutionSequence`
    (:`then_0`
      (if (`self.Is Aiming?`)
        (`self.SetActorRotation` (`KismetMathLibrary.MakeRot` 0.0 (.yaw (`KismetMathLibrary.FindLookAtRotation` (`self.K2_GetActorLocation`) (`.Location` (`GameplayStatics.BreakHitResult` (`PlayerController.GetHitResultUnderCursorByChannel` _returnvalue "TraceTypeQuery1" true)))))))))
    (:`then_1`
      ;[1 1 1] Shooting with mouse
      (`/Engine/EditorBlueprintResources/StandardMacros.Gate` true :!label _label_2
        (:`Exit`
          (`KismetSystemLibrary.Delay` (/ 1.0 7.0))
          (if (`self.Is Aiming?`)
            (`/Game/Blueprints/Weapon.Pull Trigger` _weapon)
            (else
              (`/Game/Blueprints/Weapon.Release Trigger` _weapon))))))))

(event `InputAction|Shoot`
  ;[1 1 1] Shooting with mouse
  (:`Pressed`
    (set `self.Is Shooting?` true)
    (goto _label_2 :!via `Open`))
  (:`Released`
    (set `self.Is Shooting?` false)
    (goto _label_2 :!via `Close`)))

(event `InputAction|Secondary Attack`
  ;[1 1 1] Secondary Attack
  (:`Pressed`
    (`/Game/Blueprints/Weapon.RocketFire` (`self.Weapon`))))

(fn `AddKeyBindToUMG`
  (params (VictoryInputKeyBind :type "VictoryInput Structure"))
  (bind _rebindable_main (`self.Rebindable Main`))
  (bind _returnvalue (`|CreateWidget` "/Game/UMG/KeyRebinding/ActionsRebinding/RebindKeysByElement.RebindKeysByElement_C" (`GameplayStatics.GetPlayerController` 0)))
  (set `/Game/UMG/KeyRebinding/ActionsRebinding/RebindKeysByElement.Main` _rebindable_main _returnvalue)
  (`PanelWidget.AddChild` (`/Game/UMG/KeyRebinding/ActionsRebinding/RebindKeysMain.MainScroll` _rebindable_main) (`/Game/UMG/KeyRebinding/ActionsRebinding/RebindKeysByElement.Core` _returnvalue))
  (`/Game/UMG/KeyRebinding/ActionsRebinding/RebindKeysByElement.Set Values` _returnvalue VictoryInputKeyBind))

(fn `Open Rebind Menu`
  (bind _returnvalue (`GameplayStatics.GetPlayerController` 0))
  (`VictoryBPFunctionLibrary.RemoveAllWidgetsOfClass` "/Game/UMG/KeyRebinding/ActionsRebinding/RebindKeysMain.RebindKeysMain_C")
  (bind _returnvalue_2 (`|CreateWidget` "/Game/UMG/KeyRebinding/ActionsRebinding/RebindKeysMain.RebindKeysMain_C" _returnvalue))
  (set `self.Rebindable Main` _returnvalue_2)
  (`UserWidget.AddToViewport` _returnvalue_2 0)
  (`WidgetBlueprintLibrary.SetInputMode_UIOnlyEx` _returnvalue)
  (set `PlayerController.bShowMouseCursor` true _returnvalue))

(fn `UserConstructionScript`
  ;[1 1 1] Removed this so that the viewport shows the correct paint job
)