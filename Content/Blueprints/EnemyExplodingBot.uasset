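; Exploding enemy bot for a twin-stick game that self-detonates when the player comes within attack range.
; Tick checks the distance; detonation damages the hero, fires a radial impulse, spawns an explosion and collectable orbs, and may drop a health or speed pickup.
; AffectHealth and RadialDamage add their delta to Health; death awards score and spawns a delayed explosion, without impulse or drops.
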(event `self.ReceiveBeginPlay`)

(event `self.ReceiveTick`
  (params (DeltaSeconds :type "Float (single-precision)"))
  (`self.UpdateRange`)
  (`self.Explode`))

(event `UpdateRange`
  ;[1 1 1] Update Range
  (if (< (`self.GetDistanceTo` self (`GameplayStatics.GetPlayerCharacter` 0)) (`self.AttackRange`))
    (set `self.Enemy In Range ?` true)
    (else
      (set `self.Enemy In Range ?` false))))

(event `/Game/Blueprints/iDamageable.AffectHealth`
  (params (Delta :type "Float (single-precision)"))
  (bind _capsulecomponent (`self.CapsuleComponent`))
  ;[1 1 1] Handle Death
  (`self.CalculateHealth` Delta)
  (`self.CalculateDead` :!label _label)
  (if (`self.Is Dead ?`)
    (`PrimitiveComponent.SetCollisionResponseToChannel` _capsulecomponent "ECC_WorldStatic" "ECR_Ignore")
    (`PrimitiveComponent.SetCollisionResponseToChannel` _capsulecomponent "ECC_Pawn" "ECR_Ignore")
    (bind _astwin_stick_mode (cast `/Game/Blueprints/TwinStickMode` (`GameplayStatics.GetGameMode`)))
    (`/Game/Blueprints/TwinStickMode.Increment Score` _astwin_stick_mode (`self.Score`))
    (`self.DetachFromControllerPendingDestroy`)
    (`KismetSystemLibrary.Delay` 0.2)
    (`|SpawnActorFromClass` "/Game/Blueprints/Explosion.Explosion_C" (`self.GetTransform`))
    (`self.K2_DestroyActor`)))

(event `self.ReceiveRadialDamage`
  (params (DamageReceived :type "Float (single-precision)") (DamageType :type "DamageType Object Reference") (Origin :type "Vector Structure") (HitInfo :type "HitResult Structure (by ref)") (InstigatedBy :type "Controller Object Reference") (DamageCauser :type "Actor Object Reference"))
  ;[1 1 1] Handle Death
  (`self.CalculateHealth` DamageReceived)
  (goto _label))

(event `Explode`
  (bind (_returnvalue_location _returnvalue_rotation _returnvalue_scale) (`KismetMathLibrary.BreakTransform` (`self.GetTransform`)))
  (bind _capsulecomponent (`self.CapsuleComponent`))
  ;[1 1 1] Explode
  (if (`self.Enemy In Range ?`)
    (bind _ashero_character (cast `/Game/Blueprints/HeroCharacter` (`GameplayStatics.GetPlayerCharacter` 0)))
    (message `/Game/Blueprints/iDamageable.AffectHealth` _ashero_character (`self.Damage`))
    (`PrimitiveComponent.SetCollisionResponseToChannel` _capsulecomponent "ECC_WorldStatic" "ECR_Ignore")
    (`PrimitiveComponent.SetCollisionResponseToChannel` _capsulecomponent "ECC_Pawn" "ECR_Ignore")
    (`self.DetachFromControllerPendingDestroy`)
    (`|SpawnActorFromClass` "/Game/Blueprints/Explosion.Explosion_C" (`KismetMathLibrary.MakeTransform` _returnvalue_location _returnvalue_rotation _returnvalue_scale))
    (`RadialForceComponent.FireImpulse` (`self.RadialForce`))
    (set `self.OrbSpawnLocation` _returnvalue_location)
    (for _ (range 4)
      (`|SpawnActorFromClass` "/Game/Blueprints/CollectableOrb.CollectableOrb_C" (`KismetMathLibrary.MakeTransform` (`self.OrbSpawnLocation`) (struct) (0.2 0.2 0.2)))
      (set `self.OrbSpawnLocation` (+ (`self.OrbSpawnLocation`) (40.0 10.0 0.0))))
    (if (== (`KismetMathLibrary.RandomIntegerInRange` 1 5) 5)
      (`|SpawnActorFromClass` "/Game/Blueprints/Health_PickUp.Health_PickUp_C" (`KismetMathLibrary.MakeTransform` _returnvalue_location (struct) (0.5 0.5 0.5)))
      (`self.K2_DestroyActor`)
      (elif (== (`KismetMathLibrary.RandomIntegerInRange` 1 5) 2)
        (`|SpawnActorFromClass` "/Game/Blueprints/Speed_PickUp.Speed_PickUp_C" (`KismetMathLibrary.MakeTransform` _returnvalue_location (struct) (0.5 0.5 0.5)))
        (`self.K2_DestroyActor`)
        (else
          (`self.K2_DestroyActor`))))))

(event `CalculateDead`
  ;[1 1 1] Calculate Dead
  (if (<= (`self.Health`) 0.0)
    (set `self.Is Dead ?` true)
    (else
      (set `self.Is Dead ?` false))))

(event `CalculateHealth`
  (params (Delta :type "Float (double-precision)"))
  ;[1 1 1] Calculate Health
  (set `self.Health` (+ Delta (`self.Health`))))

(fn `UserConstructionScript`)