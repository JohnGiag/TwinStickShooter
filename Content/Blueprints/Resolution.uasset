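; Resolution actor that sets the game's screen resolution on BeginPlay from a saved ResSaveGameBP slot.
; If a save exists, it applies the stored resolution with the r.SetRes console command in fullscreen or windowed mode.
; Otherwise it takes the last entry of the display adapter's resolution list as the largest, saves it as fullscreen and applies it.
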(event `self.ReceiveBeginPlay`
  (bind (_widths _heights) (`VictoryBPFunctionLibrary.OptionsMenu__GetDisplayAdapterScreenResolutions` false))
  (bind _returnvalue (`GameplayStatics.CreateSaveGameObject` "/Game/Blueprints/ResSaveGameBP.ResSaveGameBP_C"))
  (bind _asres_save_game_bp (cast `/Game/Blueprints/ResSaveGameBP` _returnvalue))
  (set `self.ResSaveInstance` _asres_save_game_bp)
  (bind _saveslotname (`/Game/Blueprints/ResSaveGameBP.SaveSlotName` _asres_save_game_bp))
  (bind _user_id (`/Game/Blueprints/ResSaveGameBP.User ID` _asres_save_game_bp))
  (bind _returnvalue_2 (`GameplayStatics.DoesSaveGameExist` _saveslotname _user_id))
  (if _returnvalue_2
    (bind _returnvalue_3 (`GameplayStatics.LoadGameFromSlot` _saveslotname _user_id))
    (bind _asres_save_game_bp_2 (cast `/Game/Blueprints/ResSaveGameBP` _returnvalue_3))
    (if (`/Game/Blueprints/ResSaveGameBP.Fullscreen?` _asres_save_game_bp_2)
      (bind _res (`/Game/Blueprints/ResSaveGameBP.Res` _asres_save_game_bp_2))
      (`KismetSystemLibrary.ExecuteConsoleCommand` (`KismetStringLibrary.Concat_StrStr` "r.SetRes " _res "f"))
      (else
        (`KismetSystemLibrary.ExecuteConsoleCommand` (`KismetStringLibrary.Concat_StrStr` "r.SetRes " _res "w"))))
    (else
      (bind _output_get (set `self.BiggestResolution` (`KismetStringLibrary.Concat_StrStr` (`KismetStringLibrary.Conv_IntToString` (`KismetArrayLibrary.Array_Get` _widths (`KismetArrayLibrary.Array_LastIndex` _widths))) "x" (`KismetStringLibrary.Conv_IntToString` (`KismetArrayLibrary.Array_Get` _heights (`KismetArrayLibrary.Array_LastIndex` _heights))))))
      (bind _returnvalue_4 (`GameplayStatics.CreateSaveGameObject` "/Game/Blueprints/ResSaveGameBP.ResSaveGameBP_C"))
      (bind _asres_save_game_bp_3 (cast `/Game/Blueprints/ResSaveGameBP` _returnvalue_4))
      (set `/Game/Blueprints/ResSaveGameBP.Res` _output_get _asres_save_game_bp_3)
      (set `/Game/Blueprints/ResSaveGameBP.Fullscreen?` true _asres_save_game_bp_3)
      (`GameplayStatics.SaveGameToSlot` _asres_save_game_bp_3 (`/Game/Blueprints/ResSaveGameBP.SaveSlotName` _asres_save_game_bp_3) (`/Game/Blueprints/ResSaveGameBP.User ID` _asres_save_game_bp_3))
      (`KismetSystemLibrary.ExecuteConsoleCommand` (`KismetStringLibrary.Concat_StrStr` "r.setRes " (`self.BiggestResolution`) "f")))))

(event `self.ReceiveActorBeginOverlap`
  (params (OtherActor :type "Actor Object Reference")))

(event `self.ReceiveTick`
  (params (DeltaSeconds :type "Float (single-precision)")))

(fn `UserConstructionScript`)