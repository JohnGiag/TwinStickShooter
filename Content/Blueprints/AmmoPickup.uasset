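; Ammo pickup actor that refills the hero character's ammo when it walks into the pickup's box.
; The box overlap prints a debug "Hello", casts the other actor to HeroCharacter and, if its ammo is below maximum, adds the pickup amount capped at that maximum.
; The pickup destroys itself only after granting ammo, so it remains when the hero is already full.
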(event `self.ReceiveBeginPlay`)

(event `self.ReceiveActorBeginOverlap`
  (params (OtherActor :type "Actor Object Reference")))

(event `self.ReceiveTick`
  (params (DeltaSeconds :type "Float (single-precision)")))

(event `self.Box.OnComponentBeginOverlap`
  (params (OtherActor :type "Actor Object Reference") (OtherComp :type "PrimitiveComponent Object Reference") (OtherBodyIndex :type Integer) (bFromSweep :type Boolean) (SweepResult :type "HitResult Structure (by ref)"))
  (`KismetSystemLibrary.PrintString` "Hello")
  (bind _ashero_character (cast `/Game/Blueprints/HeroCharacter` OtherActor))
  (`/Engine/EditorBlueprintResources/StandardMacros.IsValid` _ashero_character
    (:`Is Valid`
      (bind _ammo (`/Game/Blueprints/HeroCharacter.Ammo` _ashero_character))
      (bind _maxammo (`/Game/Blueprints/HeroCharacter.MaxAmmo` _ashero_character))
      (if (< _ammo _maxammo)
        (set `self.TempAmmo` (+ _ammo (`self.PickUpAmmoAmount`)))
        (if (> (`self.TempAmmo`) _maxammo)
          (set `self.TempAmmo` (- (`self.TempAmmo`) (- (`self.TempAmmo`) _maxammo)))
          (set `/Game/Blueprints/HeroCharacter.Ammo` (`self.TempAmmo`) _ashero_character)
          (else
            (set `/Game/Blueprints/HeroCharacter.Ammo` (`self.TempAmmo`) _ashero_character)))
        (`self.K2_DestroyActor`)))))

(fn `UserConstructionScript`)