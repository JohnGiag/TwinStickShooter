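; Projectile actor, apparently a laser shot, that damages what it hits and destroys itself on impact.
; On begin overlap, it sends its Damage through the IDamageable interface to damageable actors not tagged Friendly.
; Those hits, and overlaps with any non-damageable actor, play an attached hit sound, spawn sparks and destroy the projectile.
; Damageable actors tagged Friendly are ignored, so the projectile survives overlapping them.
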(event `self.ReceiveTick`
  (params (DeltaSeconds :type "Float (single-precision)")))

(event `self.ReceiveBeginPlay`)

(event `self.ReceiveActorBeginOverlap`
  (params (OtherActor :type "Actor Object Reference"))
  (bind (_returnvalue_location _returnvalue_rotation) (`KismetMathLibrary.BreakTransform` (`self.GetTransform`)))
  (if (`KismetSystemLibrary.DoesImplementInterface` OtherActor "/Game/Blueprints/iDamageable.iDamageable_C")
    (if (not (`self.ActorHasTag` OtherActor "Friendly"))
      (message `/Game/Blueprints/iDamageable.AffectHealth` OtherActor (`self.Damage`))
      (`GameplayStatics.PlaySoundAttached` "/Game/Audio/LaserHit.LaserHit" (`self.Projectile Collision`) :!label _label)
      (`GameplayStatics.SpawnEmitterAtLocation` "/Game/StarterContent/Particles/LaserSparks.LaserSparks" _returnvalue_location _returnvalue_rotation)
      (`self.K2_DestroyActor`))
    (else
      (goto _label))))

(fn `UserConstructionScript`)