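; Enemy turret for a twin-stick shooter that tracks and shoots at the player character within attack range.
; Each Tick it checks distance, smoothly turns the gun's yaw toward the player, and spawns projectiles from the gun socket, using a Delay to pace fire.
; Damage events add a delta to health and print it.
; At zero it relaxes collision, awards score through TwinStickMode, then spawns an explosion and destroys itself after a short delay.
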(event `self.ReceiveBeginPlay`)

(event `self.ReceiveActorBeginOverlap`
  (params (OtherActor :type "Actor Object Reference")))

(event `self.ReceiveTick`
  (params (DeltaSeconds :type "Float (single-precision)"))
  (set `self.DeltaTime` DeltaSeconds)
  (`self.Update Range`)
  (`self.Update Rotation`)
  (`self.Fire Turret Weapon`))

(event `Update Rotation`
  ;[1 1 1] Update rotation
  (if (`self.Enemy In Range ?`)
    (`SceneComponent.K2_SetWorldRotation` (`self.Gun`) (`KismetMathLibrary.RInterpTo` (`SceneComponent.K2_GetComponentRotation` (`self.Gun`)) (`KismetMathLibrary.MakeRot` 0.0 (.yaw (`KismetMathLibrary.FindLookAtRotation` (`SceneComponent.K2_GetComponentLocation` (`self.Gun`)) (`self.K2_GetActorLocation` (`GameplayStatics.GetPlayerCharacter` 0))))) (`self.DeltaTime`) (`self.RotSpeed`)) false)))

(event `Fire Turret Weapon`
  ;[1 1 1] Shoot
  (if (`self.Enemy In Range ?`)
    (`KismetSystemLibrary.Delay` (`self.FireInterval`))
    (`|SpawnActorFromClass` "/Game/Blueprints/EnemyProjectile.EnemyProjectile_C" (`SceneComponent.GetSocketTransform` (`self.Gun`) "TurretSocket" "RTS_World"))))

(event `Update Range`
  ;[1 1 1] Chek if player in range
  (if (< (`self.GetDistanceTo` self (`GameplayStatics.GetPlayerCharacter` 0)) (`self.AttackRange`))
    (set `self.Enemy In Range ?` true)
    (else
      (set `self.Enemy In Range ?` false))))

(event `/Game/Blueprints/iDamageable.AffectHealth`
  (params (Delta :type "Float (single-precision)"))
  (bind _basecollision (`self.BaseCollision`))
  ;[1 1 1] Handle Death
  (`self.CalculateHealth` Delta)
  (`self.CalculateDead` :!label _label)
  (if (`self.Is Dead?`)
    (`PrimitiveComponent.SetCollisionResponseToChannel` _basecollision "ECC_WorldStatic" "ECR_Ignore")
    (`PrimitiveComponent.SetCollisionResponseToChannel` (`self.GunCollision`) "ECC_WorldStatic" "ECR_Ignore")
    (`PrimitiveComponent.SetCollisionResponseToChannel` _basecollision "ECC_Pawn" "ECR_Ignore")
    (`PrimitiveComponent.SetCollisionResponseToChannel` (`self.GunCollision`) "ECC_Pawn" "ECR_Ignore")
    (bind _astwin_stick_mode (cast `/Game/Blueprints/TwinStickMode` (`GameplayStatics.GetGameMode`)))
    (`/Game/Blueprints/TwinStickMode.Increment Score` _astwin_stick_mode (`self.Score`))
    (`KismetSystemLibrary.Delay` 0.5)
    (`|SpawnActorFromClass` "/Game/Blueprints/Explosion.Explosion_C" (`self.GetTransform`))
    (`self.K2_DestroyActor`)))

(event `self.ReceiveRadialDamage`
  (params (DamageReceived :type "Float (single-precision)") (DamageType :type "DamageType Object Reference") (Origin :type "Vector Structure") (HitInfo :type "HitResult Structure (by ref)") (InstigatedBy :type "Controller Object Reference") (DamageCauser :type "Actor Object Reference"))
  ;[1 1 1] Handle Death
  (`self.CalculateHealth` DamageReceived)
  (goto _label))

(event `CalculateDead`
  ;[1 1 1] Calculate Dead
  (if (<= (`self.Health`) 0.0)
    (set `self.Is Dead?` true)
    (else
      (set `self.Is Dead?` false))))

(event `CalculateHealth`
  (params (Delta :type "Float (double-precision)"))
  ;[1 1 1] Calculate Health
  (bind _output_get (set `self.Health` (+ Delta (`self.Health`))))
  ;[1 1 1] Calculate Dead
  (`KismetSystemLibrary.PrintText` (`KismetTextLibrary.Conv_DoubleToText` _output_get "HalfToEven")))

(fn `UserConstructionScript`)