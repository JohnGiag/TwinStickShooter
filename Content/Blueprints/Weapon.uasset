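; Weapon actor that fires projectiles from a spawn point, gaining extra shots as orbs are counted.
; PullTrigger fires immediately and starts a looping timer at RoundsPerSecond, guarded by a DoOnce that ReleaseTrigger resets while clearing the timer.
; Fire plays the laser sound and spawns up to three projectiles at NumOfOrbs thresholds, offset along world Y rather than the muzzle's axis.
; RocketFire separately spawns a single rocket, and OrbCount increments the orb total.
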(event `self.ReceiveBeginPlay`)

(event `self.ReceiveActorBeginOverlap`
  (params (OtherActor :type "Actor Object Reference")))

(event `self.ReceiveTick`
  (params (DeltaSeconds :type "Float (single-precision)")))

(event `Pull Trigger`
  ;[1 1 1] Start and stop fire
  (`/Engine/EditorBlueprintResources/StandardMacros.DoOnce` false :!label _label
    (:`Completed`
      (`self.Fire`)
      (`KismetSystemLibrary.K2_SetTimer` null "Fire" (/ 1.0 (`self.RoundsPerSecond`)) true))))

(event `Release Trigger`
  ;[1 1 1] Start and stop fire
  (`KismetSystemLibrary.K2_ClearTimer` null "Fire")
  (goto _label :!via `Reset`))

(event `Fire`
  (bind (_returnvalue_location _returnvalue_rotation _returnvalue_scale) (`KismetMathLibrary.BreakTransform` (`SceneComponent.K2_GetComponentToWorld` (`self.ProjectileSpawnPoint`))))
  (bind _returnvalue (+ _returnvalue_location (0.0 9.0 0.0)))
  ;[1 1 1] Spawn projectile at weapon arrow
  (`GameplayStatics.PlaySoundAttached` "/Game/Audio/LaserFire.LaserFire" (`self.GunMesh`))
  (`|SpawnActorFromClass` "/Game/Blueprints/Projectile.Projectile_C" (`KismetMathLibrary.MakeTransform` _returnvalue_location _returnvalue_rotation _returnvalue_scale))
  ;[1 1 1] Extra Fire
  (if (>= (`self.NumOfOrbs`) 15)
    (`|SpawnActorFromClass` "/Game/Blueprints/Projectile.Projectile_C" (`KismetMathLibrary.MakeTransform` _returnvalue _returnvalue_rotation _returnvalue_scale))
    (if (>= (`self.NumOfOrbs`) 30)
      (`|SpawnActorFromClass` "/Game/Blueprints/Projectile.Projectile_C" (`KismetMathLibrary.MakeTransform` (+ _returnvalue (0.0 -18.0 0.0)) _returnvalue_rotation _returnvalue_scale)))))

(event `RocketFire`
  (bind (_returnvalue_location _returnvalue_rotation) (`KismetMathLibrary.BreakTransform` (`SceneComponent.K2_GetComponentToWorld` (`self.ProjectileSpawnPoint`))))
  ;[1 1 1] Rocket Fire
  (`|SpawnActorFromClass` "/Game/Blueprints/RocketProjectile.RocketProjectile_C" (`KismetMathLibrary.MakeTransform` _returnvalue_location _returnvalue_rotation (1.0 1.0 1.0))))

(event `OrbCount`
  ;[1 1 1] Orb Count
  (set `self.NumOfOrbs` (+ (`self.NumOfOrbs`) 1)))

(fn `UserConstructionScript`)