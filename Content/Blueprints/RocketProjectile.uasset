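; Rocket projectile that explodes on contact with a damageable actor, hurting nearby enemies.
; An overlap on RocketCollision passes only if the other actor implements IDamageable and a "Friendly" tag check fails.
; It then sends a negative AffectHealthMessage to every EnemyCharacter inside ExplosionCollision for area damage, spawns an explosion particle effect and destroys itself.
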(event `self.ReceiveBeginPlay`)

(event `self.RocketCollision.OnComponentBeginOverlap`
  (params (OtherActor :type "Actor Object Reference") (OtherComp :type "PrimitiveComponent Object Reference") (OtherBodyIndex :type Integer) (bFromSweep :type Boolean) (SweepResult :type "HitResult Structure (by ref)"))
  (bind (_returnvalue_location _returnvalue_rotation) (`KismetMathLibrary.BreakTransform` (`self.GetTransform`)))
  (if (`KismetSystemLibrary.DoesImplementInterface` OtherActor "/Game/Blueprints/iDamageable.iDamageable_C")
    (if (not (`self.ActorHasTag` "Friendly"))
      (for _array_element (`PrimitiveComponent.GetOverlappingActors` (`self.ExplosionCollision`) "/Game/Blueprints/EnemyCharacter.EnemyCharacter_C")
        (message `/Game/Blueprints/iDamageable.AffectHealth` _array_element -100.0))
      (`GameplayStatics.SpawnEmitterAtLocation` "/Game/StarterContent/Particles/P_Explosion.P_Explosion" _returnvalue_location _returnvalue_rotation)
      (`self.K2_DestroyActor`))))

(event `self.ReceiveActorBeginOverlap`
  (params (OtherActor :type "Actor Object Reference")))

(event `self.ReceiveTick`
  (params (DeltaSeconds :type "Float (single-precision)")))

(fn `UserConstructionScript`)