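; Enemy character for a twin-stick game that damages the hero on a looping timer while their overlap lasts.
; On death it stops blocking, awards score and detaches its controller, then after a delay spawns an explosion, collectable orbs and possibly a health or speed pickup.
; Tick pushes Health into the health bar widget every frame.
; The construction script tints the body through a dynamic material using EnemyColor.
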(event `self.ReceiveBeginPlay`)

(event `self.ReceiveActorBeginOverlap`
  (params (OtherActor :type "Actor Object Reference"))
  ;[1 1 1] Attacks with Damage Volume
  (bind _ashero_character (cast `/Game/Blueprints/HeroCharacter` OtherActor))
  (set `self.Hero` _ashero_character)
  (`KismetSystemLibrary.K2_SetTimer` null "Damage Hero" (/ 1.0 (`self.AttacksPerSecond`)) true))

(event `/Game/Blueprints/iDamageable.AffectHealth`
  (params (Delta :type "Float (single-precision)"))
  (bind (_returnvalue_location _returnvalue_rotation _returnvalue_scale) (`KismetMathLibrary.BreakTransform` (`self.GetTransform`)))
  (bind _capsulecomponent (`self.CapsuleComponent`))
  (`self.CalculateHealth` Delta)
  (if (`self.isDead`)
    (`PrimitiveComponent.SetCollisionResponseToChannel` _capsulecomponent "ECC_WorldStatic" "ECR_Ignore")
    (`PrimitiveComponent.SetCollisionResponseToChannel` _capsulecomponent "ECC_Pawn" "ECR_Ignore")
    (`SceneComponent.SetVisibility` (`self.Healthbar`) false false)
    (bind _astwin_stick_mode (cast `/Game/Blueprints/TwinStickMode` (`GameplayStatics.GetGameMode`)))
    (`/Game/Blueprints/TwinStickMode.Increment Score` _astwin_stick_mode (`self.Score`))
    (`self.DetachFromControllerPendingDestroy`)
    (`KismetSystemLibrary.Delay` 3.0)
    (`|SpawnActorFromClass` "/Game/Blueprints/Explosion.Explosion_C" (`KismetMathLibrary.MakeTransform` _returnvalue_location _returnvalue_rotation _returnvalue_scale))
    (set `self.OrbSpawnLocation` _returnvalue_location)
    (for _ (range 4)
      (`|SpawnActorFromClass` "/Game/Blueprints/CollectableOrb.CollectableOrb_C" (`KismetMathLibrary.MakeTransform` (`self.OrbSpawnLocation`) (struct) (0.2 0.2 0.2)))
      (set `self.OrbSpawnLocation` (+ (`self.OrbSpawnLocation`) (40.0 10.0 0.0))))
    (if (== (`KismetMathLibrary.RandomIntegerInRange` 1 5) 5)
      (`|SpawnActorFromClass` "/Game/Blueprints/Health_PickUp.Health_PickUp_C" (`KismetMathLibrary.MakeTransform` _returnvalue_location (struct) (0.5 0.5 0.5)))
      (`self.K2_DestroyActor`)
      (elif (== (`KismetMathLibrary.RandomIntegerInRange` 1 5) 2)
        (`|SpawnActorFromClass` "/Game/Blueprints/Speed_PickUp.Speed_PickUp_C" (`KismetMathLibrary.MakeTransform` _returnvalue_location (struct) (0.5 0.5 0.5)))
        (`self.K2_DestroyActor`)
        (else
          (`self.K2_DestroyActor`))))))

(event `Damage Hero`
  ;[1 1 1] Deal damage to the hero
  (`/Game/Blueprints/HeroCharacter.AffectHealth` (`self.Hero`) (`self.Damage`)))

(event `self.ReceiveActorEndOverlap`
  (params (OtherActor :type "Actor Object Reference"))
  ;[1 1 1] Stop the attacks
  (if (== OtherActor (`self.Hero`))
    (`KismetSystemLibrary.K2_ClearTimer` null "Damage Hero")))

(event `self.ReceiveTick`
  (params (DeltaSeconds :type "Float (single-precision)"))
  (bind _asaihealth_bar (cast `/Game/UMG/HUD/AIHealthBar` (`WidgetComponent.GetUserWidgetObject` (`self.Healthbar`))))
  (`ProgressBar.SetPercent` (`/Game/UMG/HUD/AIHealthBar.Healthbar` _asaihealth_bar) (/ (`self.Health`) 100.0)))

(fn `UserConstructionScript`
  (bind _returnvalue (`PrimitiveComponent.CreateDynamicMaterialInstance` (`self.Mesh`) 0 null))
  (bind _output_get (set `self.DynoMat` _returnvalue))
  (`MaterialInstanceDynamic.SetVectorParameterValue` _output_get "BodyColor" (`self.EnemyColor`)))